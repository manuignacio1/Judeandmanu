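; Enemy actor that hurts Megaman on contact and can be killed by shots or by his attack.
; Overlapping a BPSHot, or a Megaman whose AttackingP flag is set, destroys the enemy.
; The Box component's overlap separately calls Megaman's SubstactHealth and holds BeingDamaged true for a brief delay before clearing it, without checking whether he is attacking.
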(event `self.ReceiveActorBeginOverlap`
  (params (OtherActor :type "Actor Object Reference"))
  (`|ExecutionSequence`
    (:`then_0`
      (cast `/Game/Project/Blueprints/BPSHot` OtherActor)
      (`self.K2_DestroyActor` :!label _label))
    (:`then_1`
      (bind _asmegaman (cast `/Game/Project/Blueprints/Megaman` OtherActor))
      (if (`/Game/Project/Blueprints/Megaman.attackingP` _asmegaman)
        (goto _label)))))

(event `self.Box.OnComponentBeginOverlap`
  (params (OverlappedComponent :type "PrimitiveComponent Object Reference") (OtherActor :type "Actor Object Reference") (OtherComp :type "PrimitiveComponent Object Reference") (OtherBodyIndex :type Integer) (bFromSweep :type Boolean) (SweepResult :type "HitResult Structure (by ref)"))
  (bind _asmegaman (cast `/Game/Project/Blueprints/Megaman` OtherActor))
  (`/Game/Project/Blueprints/Megaman.Substact health` _asmegaman)
  (set `/Game/Project/Blueprints/Megaman.being damaged` true _asmegaman)
  (`KismetSystemLibrary.Delay` 0.3)
  (set `/Game/Project/Blueprints/Megaman.being damaged` false _asmegaman))

(fn `UserConstructionScript`)